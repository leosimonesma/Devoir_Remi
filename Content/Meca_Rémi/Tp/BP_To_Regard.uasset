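; BP_To_Regard is a teleporter trigger that sends any actor overlapping its Tp_Detector component to a destination actor.
; On overlap it moves the actor to the Sphere location of the first Bp_Dest_Tp found, with zero rotation, and prints a debug message.
; It then writes the player's velocity back unchanged.
; The Tp event is empty, and a ShouldTp check for the first-person character is disconnected.
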(event `self.Tp_Detector.OnComponentBeginOverlap`
  (params (OverlappedComponent :type "PrimitiveComponent Object Reference") (OtherActor :type "Actor Object Reference") (OtherComp :type "PrimitiveComponent Object Reference") (OtherBodyIndex :type Integer) (bFromSweep :type Boolean) (SweepResult :type "HitResult Structure (by ref)"))
  (bind _returnvalue (`Pawn.GetMovementComponent` (`GameplayStatics.GetPlayerCharacter` 0)))
  (bind _outactors (`GameplayStatics.GetAllActorsOfClass` "/Game/Meca_Rémi/Tp/Bp_Dest_Tp.Bp_Dest_Tp_C"))
  (`self.K2_TeleportTo` :`self` OtherActor :`DestLocation` (`SceneComponent.K2_GetComponentLocation` (`/Game/Meca_Rémi/Tp/Bp_Dest_Tp.Sphere` (`|GetArrayItem` _outactors))))
  (`KismetSystemLibrary.PrintString` "Done")
  (set `MovementComponent.Velocity` (`MovementComponent.Velocity` _returnvalue) _returnvalue))

(event `Tp`)

(fn `UserConstructionScript`)