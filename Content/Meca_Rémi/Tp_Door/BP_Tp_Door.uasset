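; BP_Tp_Door is a door Blueprint, apparently for a teleporter, that swings open and closed each time Open_Door is called.
; A FlipFlop plays or reverses the Opening timeline, whose track scaled by RotationNumber sets the Door's yaw.
; Each timeline update also moves the referenced SetVisible actor to the PortailLocation height, keeping its X and Y.
; IsOpen is set false on play and true on reverse; a branch reading it is unconnected.
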(event `Open_Door`
  (bind (_returnvalue_x _returnvalue_y) (`KismetMathLibrary.BreakVector` (`self.K2_GetActorLocation` (`self.Set_Visible`))))
  (`/Engine/EditorBlueprintResources/StandardMacros.FlipFlop`
    (:`A`
      (set `self.Is_open` false)
      (bind (_direction _newtrack_0) (`Timeline|Opening` :!label _label)
        (:`Update`
          (`SceneComponent.K2_SetRelativeRotation` (`self.Door`) (`KismetMathLibrary.MakeRotator` 0.0 0.0 (* _newtrack_0 (`self.Rotation_number`))) false false)
          (`self.K2_SetActorLocation` (`self.Set_Visible`) (`KismetMathLibrary.MakeVector` _returnvalue_x _returnvalue_y (`self.Portail location`)) false false))))
    (:`B`
      (set `self.Is_open` true)
      (goto _label :!via `Reverse`))))

(fn `UserConstructionScript`)