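; Linked portal actor that shows the view through its paired PortailLinked and teleports the first-person player between the two.
; Each tick, it moves the linked portal's scene capture to the mirrored player camera pose, rendering into a viewport-sized target fed to the plane material.
; Clip planes cut geometry behind each portal.
; When the camera crosses the plane front-to-back inside the detection volume, the character's transform, control rotation and velocity are remapped to the exit.
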(event `self.ReceiveBeginPlay`
  (bind (_returnvalue_x _returnvalue_y) (`KismetMathLibrary.BreakVector2D` (`WidgetLayoutLibrary.GetViewportSize`)))
  ;[1 1 1] Mat-Set
  (`self.SetTickGroup` "TG_PrePhysics")
  (bind _returnvalue (`KismetMaterialLibrary.CreateDynamicMaterialInstance` "/Game/Meca_Rémi/Portails/MAT_Portail.MAT_Portail"))
  (bind _output_get (set `self.MAT_Portail` _returnvalue))
  (`PrimitiveComponent.SetMaterial` (`self.Plane`) 0 _output_get)
  (bind _returnvalue_2 (`KismetRenderingLibrary.CreateRenderTarget2D` (`KismetMathLibrary.FTrunc` _returnvalue_x) (`KismetMathLibrary.FTrunc` _returnvalue_y)))
  (bind _output_get_2 (set `self.Portal_RT` _returnvalue_2))
  (`MaterialInstanceDynamic.SetTextureParameterValue` (`self.MAT_Portail`) "Texture" _output_get_2)
  (set `SceneCaptureComponent2D.TextureTarget` (`self.Portal_RT`) (`/Game/Meca_Rémi/Portails/BP_Portails.Portal_Camera` (`self.Portail_Linked`)))
  (`self.Set_Clip_planes`)
  (`MaterialInstanceDynamic.SetVectorParameterValue` (`self.MAT_Portail`) "Offset_Distance" (`KismetMathLibrary.MakeColor` (.x (* (`SceneComponent.GetForwardVector` (`self.Forward_Pointer`)) (`self.Offset`))) (.y (* (`SceneComponent.GetForwardVector` (`self.Forward_Pointer`)) (`self.Offset`))) (.z (* (`SceneComponent.GetForwardVector` (`self.Forward_Pointer`)) (`self.Offset`))))))

(event `self.ReceiveTick`
  (params (DeltaSeconds :type "Float (single-precision)"))
  (`self.Uptade_Scene_Capture`)
  (`self.Check_ViewPort_Size`)
  (`self.Should_Teleport_?`))

(fn `Check_ViewPort_Size`
  (locals (NewLocalVar :type "TextureRenderTarget2D Object Reference"))
  (bind _portal_rt (`self.Portal_RT`))
  (bind (_x _y) (`KismetMathLibrary.BreakVector2D` (`WidgetLayoutLibrary.GetViewportSize`)))
  (bind (_x_2 _y_2) (`KismetMathLibrary.BreakVector2D` (`WidgetLayoutLibrary.GetViewportSize`)))
  (if (not (and (== _x_2 (`TextureRenderTarget2D.SizeX` _portal_rt)) (== _y_2 (`TextureRenderTarget2D.SizeY` _portal_rt))))
    (`KismetSystemLibrary.PrintString` "Hello")
    (`KismetRenderingLibrary.ResizeRenderTarget2D` (`self.Portal_RT`) (`KismetMathLibrary.FTrunc` _x) (`KismetMathLibrary.FTrunc` _y))))

(fn `Is_Point_Crossing_Portal_?`
  (params (Point :type "Vector Structure") (Portal_Location :type "Vector Structure") (Portal_Normal :type "Vector Structure"))
  (returns (Return :type Boolean))
  (locals (Is_In_Front :type Boolean) (Portal_Plane :type "Plane Structure") (Is_Intersect :type Boolean :default false) (Is_Crossing :type Boolean :default false))
  (set `local.Is_In_Front` (>= (`KismetMathLibrary.Dot_VectorVector` Portal_Normal (- Point Portal_Location)) 0.0))
  (bind _output_get (set `local.Portal_Plane` (`KismetMathLibrary.MakePlaneFromPointAndNormal` (`local.Portal_Location`) (`local.Portal_Normal`))))
  (set `local.Is_Intersect` (`.ReturnValue` (`KismetMathLibrary.LinePlaneIntersection` (`self.Last_Position`) (`local.Point`) _output_get)))
  (set `local.Is_Crossing` (and (`local.Is_Intersect`) (not (`local.Is_In_Front`)) (`self.Last_In_Front`)))
  (set `self.Last_In_Front` (`local.Is_In_Front`))
  (set `self.Last_Position` (`local.Point`))
  (return (`local.Is_Crossing`)))

(fn `Set_Clip_planes`
  (bind _portal_camera (`self.Portal_Camera`))
  (`/Engine/EditorBlueprintResources/StandardMacros.IsValid` (`self.Portail_Linked`)
    (:`Is Valid`
      (set `SceneCaptureComponent2D.bEnableClipPlane` true _portal_camera)
      (set `SceneCaptureComponent2D.ClipPlaneBase` (+ (`SceneComponent.K2_GetComponentLocation` (`self.Plane`)) (* (`SceneComponent.GetForwardVector` (`self.Forward_Pointer`)) -3.0)) _portal_camera)
      (set `SceneCaptureComponent2D.ClipPlaneNormal` (`SceneComponent.GetForwardVector` (`self.Forward_Pointer`)) _portal_camera))))

(fn `Should_Teleport_?`
  (`/Engine/EditorBlueprintResources/StandardMacros.IsValid` (`|GetArrayItem` (`PrimitiveComponent.GetOverlappingActors` (`self.Player_Detection`) "/Game/FirstPerson/Blueprints/BP_FirstPersonCharacter.BP_FirstPersonCharacter_C"))
    (:`Is Valid`
      (bind _return (`self.Is_Point_Crossing_Portal_?` (`SceneComponent.K2_GetComponentLocation` (`/Game/FirstPerson/Blueprints/BP_FirstPersonCharacter.FirstPersonCamera` (cast `/Game/FirstPerson/Blueprints/BP_FirstPersonCharacter` (`GameplayStatics.GetPlayerCharacter` 0) :!pure true))) (`self.K2_GetActorLocation`) (`SceneComponent.GetForwardVector` (`self.Forward_Pointer`))))
      (if _return
        (`KismetSystemLibrary.PrintString` "TP")
        (`self.Teleport Character`)))))

(fn `Teleport Character`
  (bind _returnvalue (`self.GetTransform`))
  (bind (_returnvalue_location _returnvalue_rotation _returnvalue_scale) (`KismetMathLibrary.BreakTransform` (`self.GetTransform`)))
  (bind _returnvalue_2 (`self.GetTransform`))
  (bind _returnvalue_3 (`Pawn.GetMovementComponent` (`GameplayStatics.GetPlayerCharacter` 0)))
  (bind (_x _y _z) (`KismetMathLibrary.GetAxes` (`Controller.GetControlRotation` (`GameplayStatics.GetPlayerController` 0))))
  (bind (_x_2 _y_2 _z_2) (`KismetMathLibrary.GetAxes` (`self.K2_GetActorRotation` (`GameplayStatics.GetPlayerCharacter` 0))))
  (`self.K2_SetActorTransform` (`GameplayStatics.GetPlayerCharacter` 0) (`KismetMathLibrary.MakeTransform` (`KismetMathLibrary.TransformLocation` (`self.GetTransform` (`self.Portail_Linked`)) (`KismetMathLibrary.InverseTransformLocation` (`KismetMathLibrary.MakeTransform` _returnvalue_location _returnvalue_rotation (`KismetMathLibrary.MakeVector` (* (.x _returnvalue_scale) -1.0) (* (.y _returnvalue_scale) -1.0) (.z _returnvalue_scale))) (`self.K2_GetActorLocation` (`GameplayStatics.GetPlayerCharacter` 0)))) (`KismetMathLibrary.MakeRotationFromAxes` (`KismetMathLibrary.TransformDirection` (`self.GetTransform` (`self.Portail_Linked`)) (`KismetMathLibrary.MirrorVectorByNormal` (`KismetMathLibrary.MirrorVectorByNormal` (`KismetMathLibrary.InverseTransformDirection` _returnvalue_2 _x_2) (1.0 0.0 0.0)) (0.0 1.0 0.0))) (`KismetMathLibrary.TransformDirection` (`self.GetTransform` (`self.Portail_Linked`)) (`KismetMathLibrary.MirrorVectorByNormal` (`KismetMathLibrary.MirrorVectorByNormal` (`KismetMathLibrary.InverseTransformDirection` _returnvalue_2 _y_2) (1.0 0.0 0.0)) (0.0 1.0 0.0))) (`KismetMathLibrary.TransformDirection` (`self.GetTransform` (`self.Portail_Linked`)) (`KismetMathLibrary.MirrorVectorByNormal` (`KismetMathLibrary.MirrorVectorByNormal` (`KismetMathLibrary.InverseTransformDirection` _returnvalue_2 _z_2) (1.0 0.0 0.0)) (0.0 1.0 0.0))))) false false)
  (`Controller.SetControlRotation` (`GameplayStatics.GetPlayerController` 0) (`KismetMathLibrary.MakeRotationFromAxes` (`KismetMathLibrary.TransformDirection` (`self.GetTransform` (`self.Portail_Linked`)) (`KismetMathLibrary.MirrorVectorByNormal` (`KismetMathLibrary.MirrorVectorByNormal` (`KismetMathLibrary.InverseTransformDirection` _returnvalue _x) (1.0 0.0 0.0)) (0.0 1.0 0.0))) (`KismetMathLibrary.TransformDirection` (`self.GetTransform` (`self.Portail_Linked`)) (`KismetMathLibrary.MirrorVectorByNormal` (`KismetMathLibrary.MirrorVectorByNormal` (`KismetMathLibrary.InverseTransformDirection` _returnvalue _y) (1.0 0.0 0.0)) (0.0 1.0 0.0))) (`KismetMathLibrary.TransformDirection` (`self.GetTransform` (`self.Portail_Linked`)) (`KismetMathLibrary.MirrorVectorByNormal` (`KismetMathLibrary.MirrorVectorByNormal` (`KismetMathLibrary.InverseTransformDirection` _returnvalue _z) (1.0 0.0 0.0)) (0.0 1.0 0.0)))))
  (bind _return_value (`self.Uptade_Velocity` (`MovementComponent.Velocity` _returnvalue_3)))
  (set `MovementComponent.Velocity` _return_value _returnvalue_3))

(fn `Uptade_Scene_Capture`
  (bind _returnvalue (`self.GetTransform`))
  (bind _returnvalue_2 (`self.GetTransform` (`self.Portail_Linked`)))
  (bind (_x _y _z) (`KismetMathLibrary.BreakRotIntoAxes` (`SceneComponent.K2_GetComponentRotation` (`PlayerCameraManager.TransformComponent` (`GameplayStatics.GetPlayerCameraManager` 0)))))
  (`SceneComponent.K2_SetWorldLocationAndRotation` (`/Game/Meca_Rémi/Portails/BP_Portails.Portal_Camera` (`self.Portail_Linked`)) (`KismetMathLibrary.TransformLocation` (`self.GetTransform` (`self.Portail_Linked`)) (`KismetMathLibrary.InverseTransformLocation` (`KismetMathLibrary.MakeTransform` (.location (`self.GetTransform`)) (.rotation (`self.GetTransform`)) (`KismetMathLibrary.MakeVector` (* (.x (.scale (`self.GetTransform`))) -1.0) (* (.y (.scale (`self.GetTransform`))) -1.0) (.z (.scale (`self.GetTransform`))))) (`SceneComponent.K2_GetComponentLocation` (`PlayerCameraManager.TransformComponent` (`GameplayStatics.GetPlayerCameraManager` 0))))) (`KismetMathLibrary.MakeRotationFromAxes` (`KismetMathLibrary.TransformDirection` _returnvalue_2 (`KismetMathLibrary.MirrorVectorByNormal` (`KismetMathLibrary.MirrorVectorByNormal` (`KismetMathLibrary.InverseTransformDirection` _returnvalue _x) (1.0 0.0 0.0)) (0.0 1.0 0.0))) (`KismetMathLibrary.TransformDirection` _returnvalue_2 (`KismetMathLibrary.MirrorVectorByNormal` (`KismetMathLibrary.MirrorVectorByNormal` (`KismetMathLibrary.InverseTransformDirection` _returnvalue _y) (1.0 0.0 0.0)) (0.0 1.0 0.0))) (`KismetMathLibrary.TransformDirection` _returnvalue_2 (`KismetMathLibrary.MirrorVectorByNormal` (`KismetMathLibrary.MirrorVectorByNormal` (`KismetMathLibrary.InverseTransformDirection` _returnvalue _z) (1.0 0.0 0.0)) (0.0 1.0 0.0)))) false false))

(fn `Uptade_Velocity`
  (params (Velocity :type "Vector Structure"))
  (returns (Return_Value :type "Vector Structure"))
  (return (* (`KismetMathLibrary.TransformDirection` (`self.GetTransform` (`self.Portail_Linked`)) (`KismetMathLibrary.MirrorVectorByNormal` (`KismetMathLibrary.MirrorVectorByNormal` (`KismetMathLibrary.InverseTransformDirection` (`self.GetTransform`) (`KismetMathLibrary.Normal` Velocity)) (1.0 0.0 0.0)) (0.0 1.0 0.0))) (`KismetMathLibrary.VSize` (`local.Velocity`)))))

(fn `UserConstructionScript`)